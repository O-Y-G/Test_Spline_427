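; BP_Hebi is a snake-like chain of five paper sprite instances that travels along a spline.
; The construction script gives a provisional layout, spacing the instances by 1% of spline length from its start.
; On BeginPlay, a half-speed timeline drives distance along the spline, with each instance trailing the previous by the same spacing.
; All instances keep a fixed world-space rotation instead of following the curve's direction.
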(event `self.ReceiveBeginPlay`
  (bind _spline (`self.Spline`))
  (`TimelineComponent.SetPlayRate` (`self.Timeline_5s`) 0.5)
  (bind (_direction _alpha) (`Timeline|Timeline_5s`)
    (:`Update`
      (for _index (range 5)
        (`PaperGroupedSpriteComponent.UpdateInstanceTransform` (`self.PaperGroupedSprite`) _index (`KismetMathLibrary.MakeTransform` (`SplineComponent.GetLocationAtDistanceAlongSpline` _spline (* (+ (* _index -0.01) _alpha) (`SplineComponent.GetSplineLength` _spline)) "World") (struct :`Roll` -90.0)) false true false)))))

(fn `UserConstructionScript`
  (locals (LoopIndex :type Integer))
  (bind _spline (`self.Spline`))
  (for _index (range 5)
    (set `local.LoopIndex` _index)
    ;[1 1 1] BaseLocation（仮組）
    (`PaperGroupedSpriteComponent.UpdateInstanceTransform` (`self.PaperGroupedSprite`) (`local.LoopIndex`) (`KismetMathLibrary.MakeTransform` (`SplineComponent.GetLocationAtDistanceAlongSpline` _spline (* (`SplineComponent.GetSplineLength` _spline) (* (`local.LoopIndex`) 0.01)) "World") (struct :`Roll` -90.0)) false true false)))